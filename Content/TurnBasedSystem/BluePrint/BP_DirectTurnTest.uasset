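; BP_DirectTurnTest is a test participant for the turn-based system, tracing each step with printed messages.
; After staggered BeginPlay delays it registers with MyTurnManager and binds to its turn-changed event; the instance flagged IsFirstCharacter then starts the battle.
; When the broadcast character is itself, it simulates an action with a short delay, then calls NextTurn to pass play on.
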(event Custom|OnTurnReceived
  (params (CurrentCharacter :type Actor%20Object%20Reference))
  (Development|PrintString "OnTurnReceived Working")
  (if (== CurrentCharacter self)
    (Development|PrintString "\"It is my turn\"")
    (CallFunction|OnMyTurnStart)
    (else
      (Development|PrintString "\"Not my turn\""))))

(event EventBeginPlay
  (bind _self self)
  (Utilities|FlowControl|Delay 3.0)
  (Utilities|IsValid (Variables|Default|GetMyTurnManager)
    (:Is%20Valid
      (Development|PrintString "\"Turn Manager Connected!\"")
      (Utilities|FlowControl|Delay 2.0)
      (Class|SimpleTurnManager|AddCharacter (Variables|Default|GetMyTurnManager) _self)
      (Development|PrintString (Utilities|String|Append "\"Character \"" (Utilities|GetDisplayName _self) "\" joined!\""))
      (EventDispatchers|BindEventtoOnTurnChanged (Variables|Default|GetMyTurnManager) (delegate Custom|OnTurnReceived))
      (Development|PrintString "Bind Working")
      (Utilities|FlowControl|Delay 0.2)
      (if (Variables|Default|GetIsFirstCharacter)
        (Development|PrintString "\"Added to Turn System!\"")
        (Utilities|FlowControl|Delay 1.0)
        (Class|SimpleTurnManager|StartBattle (Variables|Default|GetMyTurnManager))
        (Development|PrintString "Start Battle")))
    (:Is%20Not%20Valid
      (Development|PrintString "\"No Turn Manager!\""))))

(event EventOnMyTurnStart
  (Development|PrintString (Utilities|String|Append "\"Character \"" "" "\" is taking action!\""))
  (Utilities|FlowControl|Delay 2.0)
  (Class|SimpleTurnManager|NextTurn (Variables|Default|GetMyTurnManager)))

(fn ConstructionScript)